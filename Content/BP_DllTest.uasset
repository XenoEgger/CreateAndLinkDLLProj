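; BP_DllTest is a test Blueprint that loads a tutorial DLL at BeginPlay and calls its exported functions to check they work.
; After importing the DLL, a sequence imports each method (inverted bool, int increment, circle area, char array), calls it with sample input and prints the result or a failure message.
; EndPlay frees the DLL, and a disconnected string-combining test is noted as experimental and crash-prone.
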(event `self.ReceiveBeginPlay`
  (bind _returnvalue (`CreateAndLinkDLLTutBFL.importDLL` "MyTutorialDLLs" "CreateAndLinkDLLTut.dll"))
  (if _returnvalue
    (`|ExecutionSequence`
      (:`then_0`
        (bind _returnvalue_2 (`CreateAndLinkDLLTutBFL.importMethodGetInvertedBool`))
        (if _returnvalue_2
          (bind _returnvalue_3 (`CreateAndLinkDLLTutBFL.getInvertedBoolFromDll` false))
          (`KismetSystemLibrary.PrintString` (`KismetStringLibrary.Concat_StrStr` "The inverted bool is: " (`KismetStringLibrary.Conv_BoolToString` _returnvalue_3)) true true (struct :`G` 0.66 :`B` 1.0 :`A` 1.0) 888.0)
          (else
            (`KismetSystemLibrary.PrintString` "Importing method Get Inverted Bool failed!" true true (struct :`R` 0.294118 :`A` 1.0) 888.0))))
      (:`then_1`
        (bind _returnvalue_4 (`CreateAndLinkDLLTutBFL.importMethodGetIntPlusPlus`))
        (if _returnvalue_4
          (bind _returnvalue_5 (`CreateAndLinkDLLTutBFL.getIntPlusPlusFromDll` 887))
          (`KismetSystemLibrary.PrintString` (`KismetStringLibrary.Concat_StrStr` "The iterated int is: " (`KismetStringLibrary.Conv_IntToString` _returnvalue_5)) true true (struct :`G` 0.66 :`B` 1.0 :`A` 1.0) 888.0)
          (else
            (`KismetSystemLibrary.PrintString` "Importing method Get Int Plus Plus failed!" true true (struct :`R` 0.294118 :`A` 1.0) 888.0))))
      (:`then_2`
        (bind _returnvalue_6 (`CreateAndLinkDLLTutBFL.importMethodGetCircleArea`))
        (if _returnvalue_6
          (bind _returnvalue_7 (`CreateAndLinkDLLTutBFL.getCircleAreaFromDll` 15.0))
          (`KismetSystemLibrary.PrintString` (`KismetStringLibrary.Concat_StrStr` "The circle area is: " (`KismetStringLibrary.Conv_DoubleToString` _returnvalue_7)) true true (struct :`G` 0.66 :`B` 1.0 :`A` 1.0) 888.0)
          (else
            (`KismetSystemLibrary.PrintString` "Importing method Get Circle Area failed!" true true (struct :`R` 0.294118 :`A` 1.0) 888.0))))
      (:`then_3`
        (bind _returnvalue_8 (`CreateAndLinkDLLTutBFL.importMethodGetCharArray`))
        (if _returnvalue_8
          (bind _returnvalue_9 (`CreateAndLinkDLLTutBFL.getCharArrayFromDll` "Hello"))
          (`KismetSystemLibrary.PrintString` (`KismetStringLibrary.Concat_StrStr` "The Char Array is: " _returnvalue_9) true true (struct :`G` 0.66 :`B` 1.0 :`A` 1.0) 888.0)
          (else
            (`KismetSystemLibrary.PrintString` "Importing method Get Char Array failed!" true true (struct :`R` 0.294118 :`A` 1.0) 888.0)))))
    (else
      (`KismetSystemLibrary.PrintString` "Importing the DLL failed!" true true (struct :`R` 0.294118 :`A` 1.0) 888.0))))

(event `self.ReceiveEndPlay`
  (params (EndPlayReason :type "EEndPlayReason Enum" :default "Destroyed"))
  (`CreateAndLinkDLLTutBFL.freeDLL`))

(fn `UserConstructionScript`)